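; Base pet Blueprint that wanders, seeks and eats food, and can be petted or picked up.
; A state variable drives Tick: while wandering it feeds the nearest food within smell radius to the AI blackboard as a target.
; Overlapping food with its sphere eats it and starts a timed Eating state.
; Petting and pickup functions toggle the blackboard's CanMove flag, restoring wandering when they end.
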(event OnComponentBeginOverlap(SphereCollision)
  (params (OverlappedComponent :type Primitive%20Component%20Object%20Reference) (OtherActor :type Actor%20Object%20Reference) (OtherComp :type Primitive%20Component%20Object%20Reference) (OtherBodyIndex :type Integer) (bFromSweep :type Boolean) (SweepResult :type Hit%20Result%20Structure%20%28by%20ref%29))
  ;[1 1 1] Eat food
  (bind _asbp_food (Utilities|Casting|CastToBP_Food OtherActor))
  (Default|EatFood _asbp_food)
  (Variables|Default|SetCurrentState "NewEnumerator2"))

(event EventBeginPlay
  (AI|Components|Blackboard|SetValueasFloat (AI|GetBlackboard 0) (Utilities|Name|MakeLiteralName "WalkRange") (Variables|Default|GetWalkRange))
  (AI|Components|Blackboard|SetValueasBool (AI|GetBlackboard 0) (Utilities|Name|MakeLiteralName "CanMove") true))

(event EventTick
  (params (DeltaSeconds :type Float%20%28single-precision%29))
  (bind _returnvalue (AI|GetBlackboard 0))
  (switch Utilities|FlowControl|Switch|SwitchonE_PetState (Variables|Default|GetCurrentState)
    (:NewEnumerator0
      ;[1 1 1] Chase food
      (bind _isfoodnearby (CallFunction|CheckFoodNearby))
      (AI|Components|Blackboard|SetValueasObject _returnvalue (Utilities|Name|MakeLiteralName "TargetActor") (Variables|Default|GetTargetFood))
      (AI|Components|Blackboard|SetValueasBool _returnvalue (Utilities|Name|MakeLiteralName "HasTarget") _isfoodnearby))
    (:NewEnumerator2
      ;[1 1 1] Eating delay
      (Utilities|FlowControl|Delay (Variables|Default|GetEatingDuration))
      (if (Utilities|Enum|Equal(Enum) (Variables|Default|GetCurrentState) "NewEnumerator2")
        (Variables|Default|SetCurrentState "NewEnumerator0")))))

(fn ConstructionScript)

(fn CheckFoodNearby
  (bind _outactors (Actor|GetAllActorsOfClass "/Game/Blueprints/BP_Food.BP_Food_C"))
  (if (and (Utilities|IsValid (.ReturnValue (Actor|FindNearestActor (Transformation|GetActorLocation) _outactors))) (< (.Distance (Actor|FindNearestActor (Transformation|GetActorLocation) _outactors)) (Variables|Default|GetSmellRadius)))
    (bind _asbp_food (Utilities|Casting|CastToBP_Food (.ReturnValue (Actor|FindNearestActor (Transformation|GetActorLocation) _outactors))))
    (Variables|Default|SetTargetFood _asbp_food)
    (return true)
    (else
      (return false))))

(fn StartPetting
  (bind _returnvalue (AI|GetBlackboard 0))
  (Variables|Default|SetCurrentState "NewEnumerator4")
  (AI|Components|Blackboard|SetValueasBool _returnvalue (Utilities|Name|MakeLiteralName "CanMove") false)
  (AI|Components|Blackboard|SetValueasBool _returnvalue (Utilities|Name|MakeLiteralName "CanMove") false))

(fn OnPickedUp
  (Variables|Default|SetCurrentState "NewEnumerator3")
  (AI|Components|Blackboard|SetValueasBool (AI|GetBlackboard 0) (Utilities|Name|MakeLiteralName "CanMove") false))

(fn OnPlacedDown
  (Variables|Default|SetCurrentState "NewEnumerator0")
  (AI|Components|Blackboard|SetValueasBool (AI|GetBlackboard 0) (Utilities|Name|MakeLiteralName "CanMove") true)
  (Development|PrintString "placeddown"))

(fn EndPetting
  (bind _returnvalue (AI|GetBlackboard 0))
  (Variables|Default|SetCurrentState "NewEnumerator0")
  (AI|Components|Blackboard|SetValueasBool _returnvalue (Utilities|Name|MakeLiteralName "CanMove") true)
  (AI|Components|Blackboard|SetValueasBool _returnvalue (Utilities|Name|MakeLiteralName "CanMove") true))