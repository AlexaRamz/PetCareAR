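; Touch interaction manager for pet care: petting, carrying and placing pets, and carrying food.
; Tap grabs food or selects a pet, a timed long press in Tick lifts the pet, and moving beyond a threshold restarts the timer and attempts petting.
; Held actors follow the deprojected mouse position until release.
; StartGame loads DT_Pets and creates WB_Main, while StartPlace spawns a chosen pet already in hand.
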(event Custom|StartGame_Event
  (Utilities|FlowControl|Sequence
    (:then_0
      (bind _outrownames (DataTable|GetDataTableRowNames "/Game/Blueprints/DT_Pets.DT_Pets"))
      (for _array_element _outrownames
        (bind _returnvalue (Utilities|GetDataTableRow "/Game/Blueprints/DT_Pets.DT_Pets" _array_element)
          (:then
            (Utilities|Array|Add (Variables|Default|GetPetsArray) _returnvalue)))))
    (:then_1
      (bind _returnvalue_2 (UserInterface|CreateWidget "/Game/UI/WB_Main.WB_Main_C" 0 self))
      (UserInterface|Viewport|AddtoViewport _returnvalue_2 0))))

(event EventTick
  (params (DeltaSeconds :type Float%20%28single-precision%29))
  (Utilities|FlowControl|Sequence
    (:then_0
      ;[1 1 1] Move picked up object
      (CallFunction|TryMoveObject))
    (:then_1
      ;[1 1 1] Pick up pet on long press
      (bind _longpresscompleted (LongPress|CheckLongPress DeltaSeconds))
      (if _longpresscompleted
        (bind _hit_actor (CallFunction|GetHitActor (Variables|Default|GetPreviousPressPosition)))
        (CallFunction|TryPickUp true _hit_actor)
        (Development|PrintString "pick up pet")))))

(event Input|TouchEvents|InputTouch
  (params (Location :type Vector) (FingerIndex :type ETouchIndex%20Enum))
  (bind _returnvalue (Math|Conversions|ToVector2D(Vector) Location))
  (:Pressed
    (bind _hit_actor (CallFunction|GetHitActor _returnvalue))
    (CallFunction|TryPickUp false _hit_actor)
    (LongPress|StartLongPress))
  (:Released
    (CallFunction|TryPlaceDown)
    (LongPress|ResetLongPress))
  (:Moved
    (bind _movingpress (CallFunction|CheckMovingPress _returnvalue))
    (if _movingpress
      (Variables|Default|SetPressElapsedTime 0.0)
      (CallFunction|TryPetting _returnvalue))))

(fn TryPickUp
  (params (CanPickUpPet :type Boolean) (Actor :type Actor%20Object%20Reference))
  (Utilities|IsValid Actor
    (:Is%20Valid
      (bind _asbp_pet_base (Utilities|Casting|CastToBP_PetBase Actor)
        (:then
          (bind _output_get (Variables|Default|SetCurrentPet _asbp_pet_base))
          (if CanPickUpPet
            (Default|OnPickedUp _output_get)
            (Variables|Default|SetPickedUpObject Actor :!label _label)
            (else
              (Variables|Default|SetPickedUpObject 0 :!label _label_2))))
        (:CastFailed
          (Variables|Default|SetCurrentPet 0)
          (Utilities|Casting|CastToBP_Food Actor
            (:then
              (goto _label))
            (:CastFailed
              (goto _label_2))))))
    (:Is%20Not%20Valid
      (Variables|Default|SetCurrentPet 0)
      (goto _label_2))))

(fn TryMoveObject
  (bind _returnvalue (Game|GetPlayerController 0))
  (bind (_locationx _locationy) (Game|Player|GetMousePosition _returnvalue))
  (bind _returnvalue_2 (Math|Vector2D|MakeVector2D _locationx _locationy))
  (bind (_worldposition _worlddirection) (Class|GameplayStatics|DeprojectScreentoWorld _returnvalue _returnvalue_2))
  (if (Utilities|IsValid (Variables|Default|GetPickedUpObject))
    (Transformation|SetActorLocation (Variables|Default|GetPickedUpObject) (+ _worldposition (* _worlddirection (Variables|Default|GetHoldingDistance))) false false)))

(fn TryPlaceDown
  (bind _currentpet (Variables|Default|GetCurrentPet))
  (Utilities|FlowControl|Sequence
    (:then_0
      (Utilities|IsValid _currentpet
        (:Is%20Valid
          (Default|OnPlacedDown _currentpet)
          (if (Variables|Default|GetPlacing)
            (Variables|Default|SetPlacing false)
            (Default|CallOnPlaceEnded)))))
    (:then_1
      (if (== (Variables|Default|GetPickedUpObject) (Variables|Default|GetNewPetTreat))
        (Development|PrintString "Take out new treat")))
    (:then_2
      (Variables|Default|SetPickedUpObject 0)
      (Development|PrintString "drop"))))

(fn CheckHitActor
  (params (ScreenLocation :type Vector%202D%20Structure))
  (CallFunction|GetHitActor ScreenLocation))

(fn StartPlace
  (params (PetIndex :type Integer))
  (bind _returnvalue (Game|SpawnActorfromClass (.SpawnActor (Utilities|Struct|BreakS_PetInfo (Utilities|Array|Get(acopy) (Variables|Default|GetPetsArray) PetIndex))) (Math|Transform|MakeTransform "0, 0, 0" "0, 0, 0" "1.000000,1.000000,1.000000") "Undefined" "MultiplyWithRoot" 0 0))
  (bind _output_get (Variables|Default|SetCurrentPet _returnvalue))
  (Variables|Default|SetPickedUpObject _output_get)
  (Variables|Default|SetPlacing true))

(fn PickUp)

(fn CheckLongPress
  (params (DeltaSeconds :type Float%20%28double-precision%29))
  (if (Variables|Default|GetLongPressStart)
    (Variables|Default|SetPressElapsedTime (+ DeltaSeconds (Variables|Default|GetPressElapsedTime)))
    (if (>= (Variables|Default|GetPressElapsedTime) (Variables|Default|GetLongPressTime))
      (LongPress|ResetLongPress)
      (return true)
      (else
        _)))
  (return false))

(fn CheckMovingPress
  (params (ScreenLocation :type Vector%202D%20Structure))
  (Utilities|FlowControl|Sequence
    (:then_0
      (bind _output_get (LocalVariables|SetMoved (> (Math|Vector|Distance2D(Vector) ScreenLocation (Variables|Default|GetPreviousPressPosition)) (Variables|Default|GetMoveThreshold)))))
    (:then_1
      (Variables|Default|SetPreviousPressPosition ScreenLocation))
    (:then_2
      (return _output_get))))

(fn ResetLongPress
  (Variables|Default|SetLongPressStart false)
  (Variables|Default|SetPressElapsedTime 0.0))

(fn StartLongPress
  (Variables|Default|SetLongPressStart true))

(fn TryPetting
  (params (ScreenLocation :type Vector%202D%20Structure))
  (bind _currentpet (Variables|Default|GetCurrentPet))
  (if (and (not (Utilities|IsValid (Variables|Default|GetPickedUpObject))) (Utilities|IsValid _currentpet))
    (bind _hit_actor (CallFunction|GetHitActor ScreenLocation))
    (Utilities|IsValid _hit_actor
      (:Is%20Valid
        (if (== _hit_actor _currentpet)
          (Default|StartPetting _currentpet)
          (else
            (Default|EndPetting _currentpet)))))))